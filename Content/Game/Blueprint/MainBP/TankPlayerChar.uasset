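; Player tank character that drives on world axes, aims its turret (Cube3) at the mouse cursor and fires projectiles.
; Tick derives turret rotation from the turret's screen position and turns the hull smoothly toward velocity.
; Any damage kills it, showing the lose widget, launching the burning turret with physics and flagging TankGI.
; E spawns an AI tank; mobile aiming and shoot-button widget logic are disconnected.
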(event Custom|ShoootEvent
  (bind _scene (Variables|Default|GetScene))
  (bind _scene_2 (Variables|Default|GetScene))
  (bind _returnvalue (Transformation|GetWorldLocation _scene))
  ;[1 1 1] Стрельба
  (Audio|SpawnSoundatLocation "/Game/Game/Sound/S_Fireshot_Classic.S_Fireshot_Classic" (Transformation|GetWorldLocation (Variables|Default|GetScene)) "0, 0, 0" 1.0 1.0 0.0 0 0)
  (Collision|LineTraceByChannel _returnvalue (+ _returnvalue (* (Math|Vector|GetForwardVector (Variables|Default|GetCube3)) 4e+03)) "TraceTypeQuery1" false 0 "None")
  ;[1 1 1] Стрельба
  (Game|SpawnActorfromClass "/Game/Game/Blueprint/MainBP/Test_B.Test_B_C" (Math|Transform|MakeTransform (Transformation|GetWorldLocation _scene_2) (Transformation|GetWorldRotation _scene_2) "1,1,1") "Undefined" 0 0)
  (Variables|Default|SetReload 0.2))

(event Game|Damage|EventAnyDamage
  (params (Damage :type Float%20%28single-precision%29) (DamageType :type Damage%20Type%20Object%20Reference) (InstigatedBy :type Controller%20Object%20Reference) (DamageCauser :type Actor%20Object%20Reference))
  (bind _cube3 (Variables|Default|GetCube3))
  (bind _returnvalue (Transformation|GetWorldLocation _cube3))
  (Variables|Default|SetHealth (- (Variables|Default|GetHealth) Damage))
  (Variables|Default|Setdeath true)
  (Utilities|FlowControl|DoOnce false
    (:Completed
      (bind _returnvalue_2 (UserInterface|CreateWidget "/Game/Game/Widget/YouLuse.YouLuse_C"))
      (UserInterface|Viewport|AddtoViewport _returnvalue_2 0)
      (Input|DisableInput 0)
      (Physics|SetSimulatePhysics _cube3 true)
      (Effects|SpawnEmitteratLocation "/Game/Realistic_Starter_VFX_Pack_Vol2/Particles/Fire/P_Fire_Big.P_Fire_Big" _returnvalue)
      (Physics|AddImpulseatLocation _cube3 "0, 0,200000.000000" _returnvalue "None")
      (Variables|/Game/Game/Blueprint/MainBP/TankGI.TankGI_C|SetPlayerDead (Variables|Default|GetGI) true))))

(event EventBeginPlay
  (bind _astank_gi (Utilities|Casting|CastToTankGI (Game|GetGameInstance)))
  (Variables|Default|SetGI _astank_gi))

(event EventTick
  (params (DeltaSeconds :type Float%20%28single-precision%29))
  (bind _returnvalue (Transformation|GetActorLocation))
  (bind _returnvalue_2 (Game|GetPlayerController 0))
  (bind _returnvalue_3 (Game|GetPlayerController 0))
  (bind _cube3 (Variables|Default|GetCube3))
  (bind (_locationx _locationy) (Game|Player|GetMousePosition _returnvalue_3))
  (bind _returnvalue_4 (Transformation|GetWorldLocation _cube3))
  (bind _screenposition (Class|GameplayStatics|ProjectWorldtoScreen _returnvalue_2 _returnvalue_4 false))
  (bind _returnvalue_5 (Math|Vector|MakeVector _locationx _locationy 0.0))
  (bind _returnvalue_6 (Math|Conversions|ToVector(Vector2D) _screenposition))
  (bind _returnvalue_7 (Math|Rotator|FindLookatRotation _returnvalue_6 _returnvalue_5))
  ;[1 1 1] Пк управление
  (if (not (Variables|Default|Getdeath))
    (Transformation|SetWorldRotation (Variables|Default|GetCube3) (Math|Rotator|MakeRotator (.roll _returnvalue_7) (.pitch _returnvalue_7) (+ (.yaw _returnvalue_7) 1.8e+02)) true false)
    (if (Math|Vector|NotEqual(Vector) (Variables|/Script/Engine.MovementComponent|GetVelocity (Variables|Character|GetCharacterMovement)) "0, 0, 0" 0.0001)
      (Transformation|SetRelativeRotation (Variables|Character|GetMesh) (Math|Interpolation|RInterpTo (Variables|/Script/Engine.SceneComponent|GetRelativeRotation (Variables|Character|GetMesh)) (Math|Rotator|FindLookatRotation _returnvalue (+ _returnvalue (* (Variables|/Script/Engine.MovementComponent|GetVelocity (Variables|Character|GetCharacterMovement)) 5e+01))) (Utilities|Time|GetWorldDeltaSeconds) 8.0) true false))))

(event Input|AxisEvents|InputAxisMoveForward
  (params (AxisValue :type Float%20%28single-precision%29))
  ;[1 1 1] Движение Вперёд
  (Pawn|Input|AddMovementInput "10.000000,0.000000, 0" (* AxisValue (Utilities|Time|GetWorldDeltaSeconds) (Variables|Default|GetSpeeed)) false))

(event Input|AxisEvents|InputAxisRotationTank
  (params (AxisValue :type Float%20%28single-precision%29))
  ;[1 1 1] вращение танка
  (Pawn|Input|AddMovementInput "0.000000,10.000000, 0" (* AxisValue (Utilities|Time|GetWorldDeltaSeconds) (Variables|Default|GetSpeeed)) false))

(event Input|AxisEvents|InputAxisX-Axis
  (params (AxisValue :type Float%20%28single-precision%29))
  ;[1 1 1] Мобильное управление
  (Variables|Default|SetAxis%20Value%20X AxisValue))

(event Input|AxisEvents|InputAxisY-Axis
  (params (AxisValue :type Float%20%28single-precision%29))
  ;[1 1 1] Мобильное управление
  (Variables|Default|SetAxis%20Value%20Y AxisValue))

(event Input|KeyboardEvents|E
  (params (Key :type Key%20Structure))
  (bind _returnvalue (Transformation|GetActorLocation))
  (bind (_x _y _z) (Math|Vector|BreakVector _returnvalue))
  (:Pressed
    (Game|SpawnActorfromClass "/Game/Game/Blueprint/MainBP/AI_Tank.AI_Tank_C" (Math|Transform|MakeTransform (Math|Vector|MakeVector (+ _x 3e+02) _y (+ _z 1e+02))) "Undefined" 0 0)))

(event Input|MouseEvents|LeftMouseButton
  (params (Key :type Key%20Structure))
  (bind _scene (Variables|Default|GetScene))
  (bind _scene_2 (Variables|Default|GetScene))
  (bind _returnvalue (Transformation|GetWorldLocation _scene))
  ;[1 1 1] Стрельба
  (:Pressed
    (Audio|SpawnSoundatLocation "/Game/Game/Sound/S_Fireshot_Classic.S_Fireshot_Classic" (Transformation|GetWorldLocation (Variables|Default|GetScene)) "0, 0, 0" 1.0 1.0 0.0 0 0)
    (Collision|LineTraceByChannel _returnvalue (+ _returnvalue (* (Math|Vector|GetForwardVector (Variables|Default|GetCube3)) 4e+03)) "TraceTypeQuery1" false 0 "None")
    ;[1 1 1] Стрельба
    (Game|SpawnActorfromClass "/Game/Game/Blueprint/MainBP/Test_B.Test_B_C" (Math|Transform|MakeTransform (Transformation|GetWorldLocation _scene_2) (Transformation|GetWorldRotation _scene_2) "1,1,1") "Undefined" 0 0)
    (Variables|Default|SetReload 0.2)))

(fn ConstructionScript)