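; Main_Char is a placeholder player character that swaps itself for either a LeopardPlayerChar or a TankPlayerChar.
; Two events, Leopard_Char and M14_Arma, each spawn their respective class at the capsule's world transform.
; Each event then has player controller 0 possess the new actor and destroys the Main_Char.
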(event Custom|M14_Arma
  (bind _returnvalue (Game|SpawnActorfromClass "/Game/Game/Blueprint/MainBP/TankPlayerChar.TankPlayerChar_C" (Transformation|GetWorldTransform (Variables|Collision|GetCapsuleComponent)) "Undefined" 0 0))
  (Pawn|Possess (Game|GetPlayerController 0) _returnvalue)
  (Actor|DestroyActor))

(event Custom|Leopard_Char
  (bind _returnvalue (Game|SpawnActorfromClass "/Game/Game/Blueprint/MainBP/LeopardPlayerChar.LeopardPlayerChar_C" (Transformation|GetWorldTransform (Variables|Collision|GetCapsuleComponent)) "Undefined" 0 0))
  (Pawn|Possess (Game|GetPlayerController 0) _returnvalue)
  (Actor|DestroyActor))

(fn ConstructionScript)