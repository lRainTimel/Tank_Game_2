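; Main menu display tank built from separate body and turret meshes, with events that switch it between the X14 and Leopard models.
; On BeginPlay it registers itself in TankGI as MainMTank.
; Tick sweeps the turret in timed bursts with pauses between, using a FlipFlop to alternate direction at a random speed.
; The yaw step is applied per frame without DeltaSeconds scaling, so turn speed depends on frame rate.
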(event Custom|Next_Tank
  (Components|StaticMesh|SetStaticMesh (Variables|Default|GetStaticMesh) "/Game/Game/Assets/Tanks/Leopard/Leopard_Body_Leopard.Leopard_Body_Leopard")
  (Components|StaticMesh|SetStaticMesh (Variables|Default|GetStaticMesh1) "/Game/Game/Assets/Tanks/Leopard/Leopard_Tower_Leopard.Leopard_Tower_Leopard"))

(event Custom|Previos%20Tank
  (Components|StaticMesh|SetStaticMesh (Variables|Default|GetStaticMesh) "/Game/Game/Assets/Tanks/T_14/x14Tank_Chassis.x14Tank_Chassis")
  (Components|StaticMesh|SetStaticMesh (Variables|Default|GetStaticMesh1) "/Game/Game/Assets/Tanks/T_14/x14Tank_Tower.x14Tank_Tower"))

(event EventBeginPlay
  (bind _astank_gi (Utilities|Casting|CastToTankGI (Game|GetGameInstance)))
  (Variables|Default|SetGI _astank_gi)
  (Variables|/Game/Game/Blueprint/MainBP/TankGI.TankGI_C|SetMainMTank (Variables|Default|GetGI) self))

(event EventTick
  (params (DeltaSeconds :type Float%20%28single-precision%29))
  (if (> (Variables|Default|Gettimer) 0.0)
    (Transformation|AddRelativeRotation (Variables|Default|GetStaticMesh1) (Math|Rotator|MakeRotator 0.0 0.0 (Variables|Default|GetRotation)) false false)
    (Variables|Default|Settimer (- (Variables|Default|Gettimer) DeltaSeconds))
    (else
      (Utilities|FlowControl|Delay 1.0)
      (Utilities|FlowControl|FlipFlop
        (:A
          (Variables|Default|SetRotation (Math|Random|RandomFloatinRange 0.1 0.8))
          (Variables|Default|Settimer 2.0))
        (:B
          (Variables|Default|SetRotation (Math|Random|RandomFloatinRange -0.8 -0.1))
          (Variables|Default|Settimer 2.0))))))

(fn ConstructionScript)