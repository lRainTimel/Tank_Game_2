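; Enemy AI tank that hunts the player, aiming its turret and halting when a forward trace sees the player.
; Tick interpolates turret yaw toward the player and drives AIMoveTo, switching to random turret spin once GameInstance reports the player dead.
; The first damage event kills it regardless of Health, flags the GameInstance, launches the turret with fire, then destroys the actor.
; Firing logic exists in Стрельба and disconnected nodes, but nothing here calls it.
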(event EventBeginPlay
  (bind _astank_gi (Utilities|Casting|CastToTankGI (Game|GetGameInstance)))
  (Variables|Default|SetGI _astank_gi))

(event EventTick
  (params (DeltaSeconds :type Float%20%28single-precision%29))
  (bind _arrow1 (Variables|Default|GetArrow1))
  (bind _returnvalue (Transformation|GetWorldLocation _arrow1))
  (if (not (Variables|Default|Getdead))
    (Variables|Default|SetReload (- (Variables|Default|GetReload) (Utilities|Time|GetWorldDeltaSeconds)))
    (if (not (Variables|/Game/Game/Blueprint/MainBP/TankGI.TankGI_C|GetPlayerDead (Variables|Default|GetGI)))
      (CallFunction|ВращениеБашни)
      (bind (_outhit _returnvalue_2) (Collision|LineTraceByChannel _returnvalue (+ _returnvalue (* (Math|Vector|GetForwardVector (Variables|Default|GetArrow1)) 1.5e+03)) "TraceTypeQuery1" false 0 "ForOneFrame"))
      (if _returnvalue_2
        (Utilities|Casting|CastToTankPlayerChar (.HitActor (Collision|BreakHitResult _outhit))
          (:then
            (Components|Movement|StopMovementImmediately (Variables|Character|GetCharacterMovement)))
          (:CastFailed
            (AI|AIMoveTo self "0, 0, 0" (Game|GetPlayerController 0) 3e+02 false)))
        (elif (> (Transformation|GetDistanceTo (Game|Player|GetPlayerPawn 0)) 1.5e+03)
          (AI|AIMoveTo self "0, 0, 0" (Game|GetPlayerController 0) 3e+02 false)))
      (else
        (Transformation|AddRelativeRotation (Variables|Default|GetCube3) (Math|Rotator|MakeRotator 0.0 0.0 (Variables|Default|GetRandom%20Rotation)) false false)
        (Utilities|FlowControl|Delay 2.0)
        (Variables|Default|SetRandom%20Rotation (Math|Random|RandomFloatinRange -1.0 1.0))))
    (else
      (Components|Movement|StopMovementImmediately (Variables|Character|GetCharacterMovement)))))

(event Game|Damage|EventAnyDamage
  (params (Damage :type Float%20%28single-precision%29) (DamageType :type Damage%20Type%20Object%20Reference) (InstigatedBy :type Controller%20Object%20Reference) (DamageCauser :type Actor%20Object%20Reference))
  (bind _cube3 (Variables|Default|GetCube3))
  (bind _returnvalue (Transformation|GetWorldLocation _cube3))
  (Variables|Default|SetHealth (- (Variables|Default|GetHealth) Damage))
  (Utilities|FlowControl|DoOnce false
    (:Completed
      (Variables|/Script/Engine.PrimitiveComponent|SetbGenerateOverlapEvents (Variables|Collision|GetCapsuleComponent) false)
      (Variables|Default|Setdead true)
      (Variables|/Game/Game/Blueprint/MainBP/TankGI.TankGI_C|SetAIDead (Variables|Default|GetGI) true)
      (Physics|SetSimulatePhysics (Variables|Default|GetCube3) true)
      (bind _returnvalue_2 (Effects|SpawnEmitteratLocation "/Game/Realistic_Starter_VFX_Pack_Vol2/Particles/Fire/P_Fire_Big.P_Fire_Big" _returnvalue))
      (Physics|AddImpulseatLocation _cube3 "0, 0,200000.000000" _returnvalue "None")
      (Utilities|FlowControl|Delay 4.0)
      (Actor|DestroyActor)
      (Components|DestroyComponent _returnvalue_2))))

(fn ConstructionScript)

(fn ВращениеБашни
  (bind _cube3 (Variables|Default|GetCube3))
  (Transformation|SetWorldRotation _cube3 (Math|Interpolation|RInterpTo (Math|Rotator|MakeRotator 0.0 0.0 (.yaw (Transformation|GetWorldRotation _cube3))) (Math|Rotator|MakeRotator 0.0 0.0 (.yaw (Math|Rotator|FindLookatRotation (Transformation|GetActorLocation) (+ (Transformation|GetActorLocation (Game|GetPlayerCharacter 0)) (Math|Vector|GetRightVector (Math|Rotator|FindLookatRotation (Transformation|GetActorLocation (Game|GetPlayerCharacter 0)) (Transformation|GetActorLocation))))))) (Utilities|Time|GetWorldDeltaSeconds) 2.0) false false))

(fn Стрельба
  (bind _arrow1 (Variables|Default|GetArrow1))
  (bind _arrow1_2 (Variables|Default|GetArrow1))
  (bind _returnvalue (Transformation|GetWorldLocation _arrow1))
  (bind (_outhit _returnvalue_2) (Collision|LineTraceByChannel _returnvalue (+ _returnvalue (* (Math|Vector|GetForwardVector (Variables|Default|GetArrow1)) 1.5e+03)) "TraceTypeQuery1" false 0 "ForOneFrame"))
  (if _returnvalue_2
    (Utilities|Casting|CastToTankPlayerChar (.HitActor (Collision|BreakHitResult _outhit)))
    (if (<= (Variables|Default|GetReload) 0.0)
      (Game|SpawnActorfromClass "/Game/Game/Blueprint/MainBP/Test_B.Test_B_C" (Math|Transform|MakeTransform (Transformation|GetWorldLocation _arrow1_2) (Transformation|GetWorldRotation _arrow1_2) "1,1,1") "Undefined" 0 0)
      (Audio|SpawnSoundatLocation "/Game/Game/Sound/S_Fireshot_Classic.S_Fireshot_Classic" (Transformation|GetWorldLocation (Variables|Default|GetArrow1)) "0, 0, 0" 1.0 1.0 0.0 0 0)
      (Variables|Default|SetReload 0.4)
      (else
        (Variables|Default|SetReload (- (Variables|Default|GetReload) (Utilities|Time|GetWorldDeltaSeconds)))))))